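; Game state that runs a short pre-match countdown and then the timed match, through to game over.
; StartGame asks BP_GameModeBase to position players; when the start count ends, pawn move speed is set and powerup spawners start.
; Countdowns loop through RepNotifies: each change updates timer widgets, and authority schedules the next delayed decrement.
; Tick also calls the start timer while the game runs and activates game-over widgets once the match finishes.
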(event Custom|StartGame
  (Variables|Default|SetgameStart true)
  (bind _asbp_game_mode_base (Utilities|Casting|CastToBP_GameModeBase (Game|GetGameMode)))
  (Default|SetPlayersLocation _asbp_game_mode_base))

(event Custom|Countdown_Match
  (Utilities|FlowControl|Delay 1.0)
  (Variables|Default|SetMatch_Countdown (- (Variables|Default|GetMatch_Countdown) 1)))

(event Custom|Start_Timer
  (if (Variables|Default|GetgameStart)
    (if (not (Variables|Default|GetfinishedStartCount))
      (Utilities|FlowControl|Delay 1.0)
      (Variables|Default|SetStartTimer (- (Variables|Default|GetStartTimer) 1)))))

(event Custom|StartGameCount
  (Variables|Default|SetMatch_Countdown 100))

(event EventBeginPlay
  (Variables|Default|SetStartTimer 5)
  (Variables|Default|SetfinishedStartCount false))

(event EventTick
  (params (DeltaSeconds :type Float%20%28single-precision%29))
  (if (Variables|Default|GetgameStart)
    (CallFunction|StartTimer)
    (if (Variables|Default|GetMatch_Finished)
      (CallFunction|UpdateMatchEnd))))

(fn ConstructionScript)

(fn UpdateMatchStart
  (bind _foundwidgets (Widget|GetAllWidgetsOfClass "/Game/Blueprints/HUD/Timer/WBP_Timer.WBP_Timer_C" false))
  (for _array_element _foundwidgets
    (Default|UpdateWidgit _array_element (Variables|Default|GetMatch_Countdown))))

(fn OnRepMatchCountdown
  (CallFunction|UpdateMatchStart)
  (Networking|SwitchHasAuthority
    (:Authority
      (if (== (Variables|Default|GetMatch_Countdown) 100)
        (CallFunction|CountdownMatch)
        (elif (== (Variables|Default|GetMatch_Countdown) 0)
          (Variables|Default|SetMatch_Finished true)
          (else
            (CallFunction|CountdownMatch)))))))

(fn UpdateMatchEnd
  (bind _foundwidgets (Widget|GetAllWidgetsOfClass "/Game/Blueprints/HUD/GameOver/WBP_GameOver.WBP_GameOver_C" false))
  (for _array_element _foundwidgets
    (Default|SetActive _array_element (Variables|Default|GetMatch_Finished))))

(fn OnRepMatchFinished)

(fn OnRepStartTimer
  (CallFunction|UpdateStartCount)
  (Networking|SwitchHasAuthority
    (:Authority
      (if (== (Variables|Default|GetStartTimer) 5)
        (CallFunction|StartTimer)
        (elif (== (Variables|Default|GetStartTimer) 0)
          (Variables|Default|SetfinishedStartCount true)
          (CallFunction|UpdateStartCount)
          (CallFunction|StartGameCount)
          (Utilities|FlowControl|Sequence
            (:then_0
              (bind _outactors (Actor|GetAllActorsOfClass "/Game/Blueprints/Player/BP_MyPlayerPawn.BP_MyPlayerPawn_C"))
              (for _array_element _outactors
                (Default|SetMoveSpeed _array_element)))
            (:then_1
              (bind _outactors_2 (Actor|GetAllActorsOfClass "/Game/Blueprints/Spawners/BP_MyPowerupSpawner.BP_MyPowerupSpawner_C"))
              (for _array_element_2 _outactors_2
                (Class|MyPowerupSpawner|StartSpawn _array_element_2))))
          (else
            (CallFunction|StartTimer)))))))

(fn UpdateStartCount
  (bind _foundwidgets (Widget|GetAllWidgetsOfClass "/Game/Blueprints/HUD/Timer/WBP_StartCount.WBP_StartCount_C" false))
  (for _array_element _foundwidgets
    (Default|UpdateWigit _array_element (Variables|Default|GetStartTimer) (Variables|Default|GetfinishedStartCount))))

(fn OnRepFinishedStartCount)