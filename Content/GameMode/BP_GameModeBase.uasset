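; Game mode that tracks lobby readiness and gives each player a separate start point.
; CheckReadyPlayers sets EveeryoneReady when ReadyPlayers equals one less than the player count.
; SetPlayersLocation moves each BP_MyPlayerPawn to an unused BP_PlayerStart through MovePlayerToStart, recording it in UsedStartPoints.
; ChoosePlayerStart returns an unused PlayerStart, tracked separately in UsedStarts; neither list is cleared here.
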(event Custom|CheckReadyPlayers
  (if (== (Variables|Default|GetreadyPlayers) (- (Utilities|Array|Length (Variables|/Script/Engine.GameStateBase|GetPlayerArray (Game|GetGameState))) 1))
    (Variables|Default|SeteveeryoneReady true)
    (else
      (Variables|Default|SeteveeryoneReady false))))

(event Custom|SetPlayersLocation
  (bind _usedstartpoints (Variables|Default|GetUsedStartPoints))
  (bind _outactors (Actor|GetAllActorsOfClass "/Game/Blueprints/Spawners/BP_PlayerStart.BP_PlayerStart_C"))
  (for _array_element (Variables|/Script/Engine.GameStateBase|GetPlayerArray (Game|GetGameState))
    (bind _asbp_my_player_pawn (Utilities|Casting|CastToBP_MyPlayerPawn (Pawn|GetControlledPawn (Game|GetPlayerController _array_element))))
    (Utilities|IsValid _asbp_my_player_pawn
      (:Is%20Valid
        (bind _array_element_2 (Utilities|Array|ForEachLoopwithBreak _outactors :!label _label)
          (:LoopBody
            (if (not (Utilities|Array|ContainsItem _usedstartpoints _array_element_2))
              (Utilities|Array|Add _usedstartpoints _array_element_2)
              (Default|MovePlayertoStart _asbp_my_player_pawn (Transformation|GetActorLocation _array_element_2) (Game|GetPlayerController _array_element))
              (goto _label Break))))))))

(event EventBeginPlay)

(event EventTick
  (params (DeltaSeconds :type Float%20%28single-precision%29)))

(fn ConstructionScript)

(fn ChoosePlayerStart
  (params (Player :type Controller%20Object%20Reference))
  (bind _usedstarts (Variables|Default|GetUsedStarts))
  (bind _outactors (Actor|GetAllActorsOfClass "/Script/Engine.PlayerStart"))
  (for _array_element _outactors
    (if (not (Utilities|Array|ContainsItem _usedstarts _array_element))
      (Utilities|Array|Add _usedstarts _array_element)
      (return _array_element))))