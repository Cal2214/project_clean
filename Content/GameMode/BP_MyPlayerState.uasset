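; BP_MyPlayerState is a player state that tracks whether its player is ready.
; SetReady and RemoveReady set IsReady, adjust the ReadyPlayers count on BP_GameModeBase and call its CheckReadyPlayers.
; RemoveReady decrements through the game mode reference cast in SetReady, so it relies on SetReady having run first.
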(event Custom|SetReady
  (Variables|Default|SetisReady true)
  (bind _asbp_game_mode_base (Utilities|Casting|CastToBP_GameModeBase (Game|GetGameMode)))
  (bind _result (Math|Integer|IncrementInt (Variables|/Game/GameMode/BP_GameModeBase.BP_GameModeBase_C|GetreadyPlayers _asbp_game_mode_base))
    (:%20%20
      (Variables|/Game/GameMode/BP_GameModeBase.BP_GameModeBase_C|SetreadyPlayers _asbp_game_mode_base _result)
      (Default|CheckReadyPlayers _asbp_game_mode_base))))

(event Custom|RemoveReady
  (Variables|Default|SetisReady false)
  (bind _asbp_game_mode_base (Utilities|Casting|CastToBP_GameModeBase (Game|GetGameMode)))
  (bind _result (Math|Integer|DecrementInt (Variables|/Game/GameMode/BP_GameModeBase.BP_GameModeBase_C|GetreadyPlayers (stale Custom|SetReady _asbp_game_mode_base)))
    (:%20%20
      (Variables|/Game/GameMode/BP_GameModeBase.BP_GameModeBase_C|SetreadyPlayers _asbp_game_mode_base _result)
      (Default|CheckReadyPlayers _asbp_game_mode_base))))

(event EventBeginPlay)

(event EventTick
  (params (DeltaSeconds :type Float%20%28single-precision%29)))

(fn ConstructionScript)