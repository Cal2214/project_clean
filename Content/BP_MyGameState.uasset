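; Game State Blueprint that runs a match countdown and shows it on timer widgets.
; BeginPlay initializes MatchCountdown, and its RepNotify pushes each new value to every WBP_Timer widget.
; On authority, the RepNotify also calls a delayed one-second decrement, forming a self-driving loop through the variable's own notify instead of a timer or Tick.
; At zero the authority stops counting and only prints a GameOver debug message.
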(event Custom|Countdown_Match
  (Utilities|FlowControl|Delay 1.0)
  (Variables|Default|SetMatch_Countdown (- (Variables|Default|GetMatch_Countdown) 1)))

(event EventBeginPlay
  (Variables|Default|SetMatch_Countdown 100))

(event EventTick
  (params (DeltaSeconds :type Float%20%28single-precision%29)))

(fn ConstructionScript)

(fn OnRepMatchCountdown
  (CallFunction|UpdateMatchStart)
  (Networking|SwitchHasAuthority
    (:Authority
      (if (== (Variables|Default|GetMatch_Countdown) 100)
        (CallFunction|CountdownMatch)
        (elif (== (Variables|Default|GetMatch_Countdown) 0)
          (Development|PrintString "GameOver" true true "(R=1.000000,G=0.000000,B=0.846239,A=1.000000)")
          (else
            (CallFunction|CountdownMatch)))))))

(fn UpdateMatchStart
  (bind _foundwidgets (Widget|GetAllWidgetsOfClass "/Game/Blueprints/HUD/Timer/WBP_Timer.WBP_Timer_C" false))
  (for _array_element _foundwidgets
    (Default|UpdateWidgit _array_element (Variables|Default|GetMatch_Countdown))))