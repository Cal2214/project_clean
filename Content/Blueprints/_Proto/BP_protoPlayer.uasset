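; Prototype player actor that moves continuously in four directions via WASD without direct reversal, collecting BP_Dirt for score.
; Key presses set direction flags that Tick turns into per-frame location offsets, not scaled by delta time.
; Box overlap adds dirt points, and BeginPlay creates the HUD widget.
; GetPowerUp fills two slots with speed or size boosts, which Q and E trigger temporarily through delay-based resets.
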(event OnComponentBeginOverlap(Box)
  (params (OverlappedComponent :type Primitive%20Component%20Object%20Reference) (OtherActor :type Actor%20Object%20Reference) (OtherComp :type Primitive%20Component%20Object%20Reference) (OtherBodyIndex :type Integer) (bFromSweep :type Boolean) (SweepResult :type Hit%20Result%20Structure%20%28by%20ref%29))
  (bind _asbp_dirt (Utilities|Casting|CastToBP_Dirt OtherActor))
  (Variables|Default|SetScore (+ (Variables|/Game/Blueprints/_Proto/BP_Dirt.BP_Dirt_C|GetPoints _asbp_dirt) (Variables|Default|GetScore)))
  (Default|CollectDirt _asbp_dirt))

(event Custom|MoveUp
  (bind _returnvalue (Transformation|GetActorLocation))
  (Transformation|SetActorLocation (Math|Vector|MakeVector (+ (.x _returnvalue) (.x (* (Transformation|GetActorForwardVector) (Variables|Default|GetmoveSpeed)))) (.y _returnvalue) (.z _returnvalue)) false false))

(event Custom|MoveDown
  (bind _returnvalue (Transformation|GetActorLocation))
  (Transformation|SetActorLocation (Math|Vector|MakeVector (+ (.x _returnvalue) (.x (* (* (Transformation|GetActorForwardVector) (Variables|Default|Getmultiply)) (Variables|Default|GetmoveSpeed)))) (.y _returnvalue) (.z _returnvalue)) false false))

(event Custom|MoveRight
  (bind _returnvalue (Transformation|GetActorLocation))
  (Transformation|SetActorLocation (Math|Vector|MakeVector (.x _returnvalue) (+ (.y _returnvalue) (.y (* (Transformation|GetActorRightVector) (Variables|Default|GetmoveSpeed)))) (.z _returnvalue)) false false))

(event Custom|MoveLeft
  (bind _returnvalue (Transformation|GetActorLocation))
  (Transformation|SetActorLocation (Math|Vector|MakeVector (.x _returnvalue) (+ (.y _returnvalue) (.y (* (* (Transformation|GetActorRightVector) (Variables|Default|Getmultiply)) (Variables|Default|GetmoveSpeed)))) (.z _returnvalue)) false false))

(event Custom|DirtRef
  (bind _outactors (Actor|GetAllActorsOfClass "/Game/Blueprints/_Proto/BP_Dirt.BP_Dirt_C"))
  (Variables|Default|SetBP_Dirt (Utilities|Array|Get(acopy) _outactors)))

(event Custom|UsePowerUP
  (bind _staticmesh (Variables|Default|GetStaticMesh))
  (bind _staticmesh_2 (Variables|Default|GetStaticMesh))
  (if (Variables|Default|GetusePowerUp1)
    (Variables|Default|SetusePowerUp1 false)
    (if (Variables|Default|GethasPowerUP1)
      (if (Variables|Default|GethasSpeedLeft)
        (Variables|Default|SetmoveSpeed 1e+01)
        (CallFunction|RemoveLeftPowerUp)
        (Variables|Default|SethasSpeedLeft false)
        (Rendering|Material|SetMaterial (Variables|Default|GetStaticMesh) 0 "/AnimationSharing/AnimSharingBlue.AnimSharingBlue")
        (Utilities|FlowControl|Delay 1e+01)
        (Variables|Default|SetmoveSpeed 5.0)
        (Rendering|Material|SetMaterial (Variables|Default|GetStaticMesh) 0 "/Engine/EngineMaterials/WorldGridMaterial.WorldGridMaterial")
        (elif (Variables|Default|GethasSizeLeft)
          (Transformation|SetWorldScale3D _staticmesh_2 "0.700000,0.700000,0.300000")
          (CallFunction|RemoveLeftPowerUp)
          (Variables|Default|SethasSizeLeft false)
          (Utilities|FlowControl|Delay 1e+01)
          (Transformation|SetWorldScale3D _staticmesh_2 "0.350000,0.350000,0.300000"))))
    (elif (Variables|Default|GetusePowerUp2)
      (Variables|Default|SetusePowerUp2 false)
      (if (Variables|Default|GethasPowerUP2)
        (if (Variables|Default|GethasSpeedRight)
          (Variables|Default|SetmoveSpeed 1e+01)
          (CallFunction|RemoveRightPowerUp)
          (Variables|Default|SethasSpeedRight false)
          (Rendering|Material|SetMaterial (Variables|Default|GetStaticMesh) 0 "/AnimationSharing/AnimSharingBlue.AnimSharingBlue")
          (Utilities|FlowControl|Delay 1e+01)
          (Variables|Default|SetmoveSpeed 5.0)
          (Rendering|Material|SetMaterial (Variables|Default|GetStaticMesh) 0 "/Engine/EngineMaterials/WorldGridMaterial.WorldGridMaterial")
          (elif (Variables|Default|GethasSizeRight)
            (Transformation|SetWorldScale3D _staticmesh "0.700000,0.700000,0.300000")
            (CallFunction|RemoveRightPowerUp)
            (Variables|Default|SethasSizeRight false)
            (Utilities|FlowControl|Delay 1e+01)
            (Transformation|SetWorldScale3D _staticmesh "0.350000,0.350000,0.300000")))))))

(event Custom|HUD
  (bind _returnvalue (UserInterface|CreateWidget "/Game/Blueprints/_Proto/WBP_HUD.WBP_HUD_C"))
  (bind _output_get (Variables|Default|SetWBP_HUD _returnvalue))
  (UserInterface|Viewport|AddtoViewport _output_get 0))

(event Custom|GetPowerUp
  (params (IsSpeed :type Boolean) (isSize :type Boolean))
  (Utilities|FlowControl|Sequence
    (:then_0
      (if (Variables|Default|GethasPowerUP1)
        (if (not (Variables|Default|GethasPowerUP2))
          (Variables|Default|SethasPowerUP2 true)
          (if IsSpeed
            (Variables|Default|SetSpeed true)
            (Variables|Default|SethasSpeedRight true)
            (Variables|Default|SetSpeedImage (Variables|Default|GetSpeedImage))
            (elif isSize
              (Variables|Default|SetSize true)
              (Variables|Default|SethasSizeRight true)
              (Variables|Default|SetSizeImage "/Engine/EngineResources/AICON-Red.AICON-Red"))))
        (else
          (Variables|Default|SethasPowerUP1 true)
          (if IsSpeed
            (Variables|Default|SetSpeed true)
            (Variables|Default|SethasSpeedLeft true)
            (Variables|Default|SetSpeedImage (Variables|Default|GetSpeedImage))
            (elif isSize
              (Variables|Default|SetSize true)
              (Variables|Default|SethasSizeLeft true)
              (Variables|Default|SetSizeImage "/Engine/EngineResources/AICON-Red.AICON-Red"))))))
    (:then_1
      (if (and (Variables|Default|GethasPowerUP1) (Variables|Default|GethasPowerUP2))
        (Variables|Default|SethasMaxPowerup true)))))

(event Custom|RemoveLeftPowerUp
  (Variables|Default|SethasPowerUP1 false)
  (Variables|Default|SethasMaxPowerup false))

(event Custom|RemoveRightPowerUp
  (Variables|Default|SethasPowerUP2 false)
  (Variables|Default|SethasMaxPowerup false))

(event EventBeginPlay
  (CallFunction|HUD))

(event Collision|EventActorBeginOverlap
  (params (OtherActor :type Actor%20Object%20Reference)))

(event EventTick
  (params (DeltaSeconds :type Float%20%28single-precision%29))
  (switch int (Variables|Default|GetDirection)
    (:1
      (if (Variables|Default|GetisUp)
        (Variables|Default|SetisRight false)
        (Variables|Default|SetisDown false)
        (Variables|Default|SetisLeft false)
        (CallFunction|MoveUp)))
    (:2
      (if (Variables|Default|GetisDown)
        (Variables|Default|SetisRight false)
        (Variables|Default|SetisUp false)
        (Variables|Default|SetisLeft false)
        (CallFunction|MoveDown)))
    (:3
      (if (Variables|Default|GetisRight)
        (Variables|Default|SetisDown false)
        (Variables|Default|SetisUp false)
        (Variables|Default|SetisLeft false)
        (CallFunction|MoveRight)))
    (:4
      (if (Variables|Default|GetisLeft)
        (Variables|Default|SetisRight false)
        (Variables|Default|SetisUp false)
        (Variables|Default|SetisDown false)
        (CallFunction|MoveLeft)))))

(event Input|KeyboardEvents|D
  (params (Key :type Key%20Structure :default "None"))
  (:Pressed
    (if (not (Variables|Default|GetisLeft))
      (Variables|Default|SetisRight true)
      (Variables|Default|SetDirection 3))))

(event Input|KeyboardEvents|W
  (params (Key :type Key%20Structure :default "None"))
  (:Pressed
    (if (not (Variables|Default|GetisDown))
      (Variables|Default|SetisUp true)
      (Variables|Default|SetDirection 1))))

(event Input|KeyboardEvents|S
  (params (Key :type Key%20Structure :default "None"))
  (:Pressed
    (if (not (Variables|Default|GetisUp))
      (Variables|Default|SetisDown true)
      (Variables|Default|SetDirection 2))))

(event Input|KeyboardEvents|A
  (params (Key :type Key%20Structure :default "None"))
  (:Pressed
    (if (not (Variables|Default|GetisRight))
      (Variables|Default|SetisLeft true)
      (Variables|Default|SetDirection 4))))

(event Input|KeyboardEvents|Q
  (params (Key :type Key%20Structure :default "None"))
  (:Pressed
    (Variables|Default|SetusePowerUp1 true)
    (CallFunction|UsePowerUP)))

(event Input|KeyboardEvents|E
  (params (Key :type Key%20Structure :default "None"))
  (:Pressed
    (Variables|Default|SetusePowerUp2 true)
    (CallFunction|UsePowerUP)))

(fn ConstructionScript)