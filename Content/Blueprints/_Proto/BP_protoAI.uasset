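; Prototype AI actor that seeks the nearest BP_Dirt, collects it on overlap and adds its points to a score.
; Tick moves it along the dominant X or Y axis toward that target, picking a new nearest dirt after each pickup.
; Overlapping BP_Obsticals triggers a random perpendicular detour for a second before seeking resumes.
; It holds two power-up slots for timed speed or size boosts, which NotiPowerUp spends after a random delay.
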(event OnComponentBeginOverlap(Box)
  (params (OverlappedComponent :type Primitive%20Component%20Object%20Reference) (OtherActor :type Actor%20Object%20Reference) (OtherComp :type Primitive%20Component%20Object%20Reference) (OtherBodyIndex :type Integer) (bFromSweep :type Boolean) (SweepResult :type Hit%20Result%20Structure%20%28by%20ref%29))
  (bind _asbp_dirt (Utilities|Casting|CastToBP_Dirt OtherActor))
  (Variables|Default|SetScore (+ (Variables|/Game/Blueprints/_Proto/BP_Dirt.BP_Dirt_C|GetPoints _asbp_dirt) (Variables|Default|GetScore)))
  (Default|CollectDirt _asbp_dirt)
  (CallFunction|GetDirection))

(event OnComponentBeginOverlap(CheckOb)
  (params (OverlappedComponent :type Primitive%20Component%20Object%20Reference) (OtherActor :type Actor%20Object%20Reference) (OtherComp :type Primitive%20Component%20Object%20Reference) (OtherBodyIndex :type Integer) (bFromSweep :type Boolean) (SweepResult :type Hit%20Result%20Structure%20%28by%20ref%29))
  (Utilities|Casting|CastToBP_Obsticals OtherActor)
  (Variables|Default|SetChangeDirection true)
  (CallFunction|Change))

(event OnComponentEndOverlap(CheckOb)
  (params (OverlappedComponent :type Primitive%20Component%20Object%20Reference) (OtherActor :type Actor%20Object%20Reference) (OtherComp :type Primitive%20Component%20Object%20Reference) (OtherBodyIndex :type Integer))
  (Utilities|Casting|CastToBP_Obsticals OtherActor))

(event Custom|MoveUp
  (bind _self self)
  (bind _returnvalue (Transformation|GetActorLocation _self))
  (if (Variables|Default|GetisUp)
    (Transformation|SetActorLocation _self (Math|Vector|MakeVector (+ (.x _returnvalue) (.x (* (Transformation|GetActorForwardVector _self) (Variables|Default|GetmoveSpeed)))) (.y _returnvalue) (.z _returnvalue)) false false)))

(event Custom|MoveDown
  (bind _self self)
  (bind _returnvalue (Transformation|GetActorLocation _self))
  (if (Variables|Default|GetisDown)
    (Transformation|SetActorLocation _self (Math|Vector|MakeVector (+ (.x _returnvalue) (.x (* (* (Transformation|GetActorForwardVector _self) (Variables|Default|Getmultiply)) (Variables|Default|GetmoveSpeed)))) (.y _returnvalue) (.z _returnvalue)) false false)))

(event Custom|GetDirection
  (bind _returnvalue (Transformation|GetActorLocation))
  (bind _dirt (Variables|Default|GetDirt))
  (bind (_distance _returnvalue_2) (Actor|FindNearestActor _returnvalue _dirt))
  (CallFunction|DirtRef)
  (Variables|Default|SetDistance _distance)
  (Variables|Default|SetClosestDirt _returnvalue_2)
  (CallFunction|MovetoDirection))

(event Custom|DirtRef
  (bind _outactors (Actor|GetAllActorsOfClass "/Game/Blueprints/_Proto/BP_Dirt.BP_Dirt_C"))
  (Variables|Default|SetDirt _outactors))

(event Custom|MoveToDirection
  (bind _returnvalue (Transformation|GetActorLocation))
  (bind _closestdirt (Variables|Default|GetClosestDirt))
  (bind _returnvalue_2 (Transformation|GetActorLocation _closestdirt))
  (bind _returnvalue_3 (- _returnvalue_2 _returnvalue))
  (bind _returnvalue_4 (Math|Vector|Normalize _returnvalue_3 1.0))
  (bind (_x _y) (Math|Vector|BreakVector _returnvalue_4))
  (Utilities|IsValid (Variables|Default|GetClosestDirt)
    (:Is%20Valid
      (if (> (Math|Float|Absolute(Float) _x) (Math|Float|Absolute(Float) _y))
        (if (> _x 0.0)
          (Variables|Default|SetDirection 0)
          (else
            (Variables|Default|SetDirection 1)))
        (elif (> _y 0.0)
          (Variables|Default|SetDirection 2)
          (else
            (Variables|Default|SetDirection 3)))))
    (:Is%20Not%20Valid
      (CallFunction|GetDirection))))

(event Custom|MoveRight
  (bind _self self)
  (bind _returnvalue (Transformation|GetActorLocation _self))
  (if (Variables|Default|GetisRight)
    (Transformation|SetActorLocation _self (Math|Vector|MakeVector (.x _returnvalue) (+ (.y _returnvalue) (.y (* (Transformation|GetActorRightVector _self) (Variables|Default|GetmoveSpeed)))) (.z _returnvalue)) false false)))

(event Custom|MoveLeft
  (bind _self self)
  (bind _returnvalue (Transformation|GetActorLocation _self))
  (if (Variables|Default|GetisLeft)
    (Transformation|SetActorLocation _self (Math|Vector|MakeVector (.x _returnvalue) (+ (.y _returnvalue) (.y (* (* (Transformation|GetActorRightVector _self) (Variables|Default|Getmultiply)) (Variables|Default|GetmoveSpeed)))) (.z _returnvalue)) false false)))

(event Custom|Change
  (if (Variables|Default|GetisUp)
    (Utilities|FlowControl|DoOnce false :!label _label
      (:Completed
        (switch int (Math|Random|RandomInteger 2)
          (:0
            (Variables|Default|SetDirection 2)
            (Variables|Default|SetnewDirection true)
            (Utilities|FlowControl|Delay 1.0)
            (Variables|Default|SetChangeDirection false)
            (Variables|Default|SetnewDirection false)
            (goto _label Reset))
          (:1
            (Variables|Default|SetDirection 3)
            (Variables|Default|SetnewDirection true)
            (Utilities|FlowControl|Delay 1.0)
            (Variables|Default|SetChangeDirection false)
            (Variables|Default|SetnewDirection false)
            (goto _label Reset)))))
    (elif (Variables|Default|GetisDown)
      (Utilities|FlowControl|DoOnce false :!label _label_2
        (:Completed
          (switch int (Math|Random|RandomInteger 2)
            (:0
              (Variables|Default|SetDirection 2)
              (Variables|Default|SetnewDirection true)
              (Utilities|FlowControl|Delay 1.0)
              (Variables|Default|SetChangeDirection false)
              (Variables|Default|SetnewDirection false)
              (goto _label_2 Reset))
            (:1
              (Variables|Default|SetDirection 3)
              (Variables|Default|SetnewDirection true)
              (Utilities|FlowControl|Delay 1.0)
              (Variables|Default|SetChangeDirection false)
              (Variables|Default|SetnewDirection false)
              (goto _label_2 Reset)))))
      (elif (Variables|Default|GetisRight)
        (Utilities|FlowControl|DoOnce false :!label _label_3
          (:Completed
            (switch int (Math|Random|RandomInteger 2)
              (:0
                (Variables|Default|SetDirection 0)
                (Variables|Default|SetnewDirection true)
                (Utilities|FlowControl|Delay 1.0)
                (Variables|Default|SetChangeDirection false)
                (Variables|Default|SetnewDirection false)
                (goto _label_3 Reset))
              (:1
                (Variables|Default|SetDirection 1)
                (Variables|Default|SetnewDirection true)
                (Utilities|FlowControl|Delay 1.0)
                (Variables|Default|SetChangeDirection false)
                (Variables|Default|SetnewDirection false)
                (goto _label_3 Reset)))))
        (elif (Variables|Default|GetisLeft)
          (Utilities|FlowControl|DoOnce false :!label _label_4
            (:Completed
              (switch int (Math|Random|RandomInteger 2)
                (:0
                  (Variables|Default|SetDirection 0)
                  (Variables|Default|SetnewDirection true)
                  (Utilities|FlowControl|Delay 1.0)
                  (Variables|Default|SetChangeDirection false)
                  (Variables|Default|SetnewDirection false)
                  (goto _label_4 Reset))
                (:1
                  (Variables|Default|SetDirection 1)
                  (Variables|Default|SetnewDirection true)
                  (Utilities|FlowControl|Delay 1.0)
                  (Variables|Default|SetChangeDirection false)
                  (Variables|Default|SetnewDirection false)
                  (goto _label_4 Reset))))))))))

(event Custom|GetPowerup
  (params (isSpeed :type Boolean) (isSize :type Boolean))
  (Utilities|FlowControl|Sequence
    (:then_0
      (if (Variables|Default|GethasPowerUP1)
        (if (not (Variables|Default|GethasPowerUP2))
          (Variables|Default|SethasPowerUP2 true)
          (if isSpeed
            (Variables|Default|SetSpeed true)
            (Variables|Default|SethasSpeedRight true)
            (elif isSize
              (Variables|Default|SetSize true)
              (Variables|Default|SethasSizeRight true))))
        (else
          (Variables|Default|SethasPowerUP1 true)
          (if isSpeed
            (Variables|Default|SetSpeed true)
            (Variables|Default|SethasSpeedLeft true)
            (elif isSize
              (Variables|Default|SetSize true)
              (Variables|Default|SethasSizeLeft true))))))))

(event Custom|UsePowerUp
  (bind _staticmesh (Variables|Default|GetStaticMesh))
  (bind _staticmesh_2 (Variables|Default|GetStaticMesh))
  (if (Variables|Default|GetusePowerUp1)
    (Variables|Default|SetusePowerUp1 false)
    (if (Variables|Default|GethasPowerUP1)
      (if (Variables|Default|GethasSpeedLeft)
        (Variables|Default|SetmoveSpeed 1e+01)
        (Variables|Default|SethasSpeedLeft false)
        (Rendering|Material|SetMaterial (Variables|Default|GetStaticMesh) 0 "/AnimationSharing/AnimSharingBlue.AnimSharingBlue")
        (Utilities|FlowControl|Delay 1e+01)
        (Variables|Default|SetmoveSpeed 5.0)
        (Rendering|Material|SetMaterial (Variables|Default|GetStaticMesh) 0 "/Engine/EngineMaterials/WorldGridMaterial.WorldGridMaterial")
        (elif (Variables|Default|GethasSizeLeft)
          (Transformation|SetWorldScale3D _staticmesh_2 "0.700000,0.700000,0.300000")
          (Variables|Default|SethasSizeLeft false)
          (Utilities|FlowControl|Delay 1e+01)
          (Transformation|SetWorldScale3D _staticmesh_2 "0.350000,0.350000,0.300000"))))
    (elif (Variables|Default|GetusePowerUp2)
      (Variables|Default|SetusePowerUp2 false)
      (if true
        (if (Variables|Default|GethasSpeedRight)
          (Variables|Default|SetmoveSpeed 1e+01)
          (Variables|Default|SethasSpeedRight false)
          (Rendering|Material|SetMaterial (Variables|Default|GetStaticMesh) 0 "/AnimationSharing/AnimSharingBlue.AnimSharingBlue")
          (Utilities|FlowControl|Delay 1e+01)
          (Variables|Default|SetmoveSpeed 5.0)
          (Rendering|Material|SetMaterial (Variables|Default|GetStaticMesh) 0 "/Engine/EngineMaterials/WorldGridMaterial.WorldGridMaterial")
          (elif (Variables|Default|GethasSizeRight)
            (Transformation|SetWorldScale3D _staticmesh "0.700000,0.700000,0.300000")
            (Variables|Default|SethasSizeRight false)
            (Utilities|FlowControl|Delay 1e+01)
            (Transformation|SetWorldScale3D _staticmesh "0.350000,0.350000,0.300000")))))))

(event Custom|NotiPowerUp
  (Utilities|FlowControl|Delay (Math|Random|RandomFloatinRange 1.0 2e+01))
  (if (and (Variables|Default|GethasPowerUP1) (Variables|Default|GethasPowerUP2))
    (Variables|Default|SethasMaxPowerUp true))
  (if (Math|Random|RandomBool)
    (if (Variables|Default|GethasPowerUP1)
      (Variables|Default|SetusePowerUp1 true)
      (CallFunction|UsePowerUp)
      (Variables|Default|SetusePowerUp1 false)
      (Variables|Default|SethasPowerUP1 false)
      (Variables|Default|SethasMaxPowerUp false)
      (elif (Variables|Default|GethasPowerUP2)
        (Variables|Default|SetusePowerUp2 true)
        (CallFunction|UsePowerUp)
        (Variables|Default|SetusePowerUp2 false)
        (Variables|Default|SethasPowerUP2 false)
        (Variables|Default|SethasMaxPowerUp false)))
    (elif (Variables|Default|GethasPowerUP2)
      (Variables|Default|SetusePowerUp2 true)
      (CallFunction|UsePowerUp)
      (Variables|Default|SetusePowerUp2 false)
      (Variables|Default|SethasPowerUP2 false)
      (Variables|Default|SethasMaxPowerUp false)
      (else
        (Variables|Default|SetusePowerUp1 true)
        (CallFunction|UsePowerUp)
        (Variables|Default|SetusePowerUp1 false)
        (Variables|Default|SethasPowerUP1 false)
        (Variables|Default|SethasMaxPowerUp false)))))

(event EventTick
  (params (DeltaSeconds :type Float%20%28single-precision%29))
  (if (Variables|Default|GetChangeDirection)
    (if (Variables|Default|GetnewDirection)
      (switch int (Variables|Default|GetDirection) :!label _label
        (:0
          (CallFunction|MoveUp)
          (Variables|Default|SetisUp true)
          (Variables|Default|SetisDown false)
          (Variables|Default|SetisRight false)
          (Variables|Default|SetisLeft false))
        (:1
          (CallFunction|MoveDown)
          (Variables|Default|SetisDown true)
          (Variables|Default|SetisUp false)
          (Variables|Default|SetisRight false)
          (Variables|Default|SetisLeft false))
        (:2
          (CallFunction|MoveRight)
          (Variables|Default|SetisRight true)
          (Variables|Default|SetisDown false)
          (Variables|Default|SetisUp false)
          (Variables|Default|SetisLeft false))
        (:3
          (CallFunction|MoveLeft)
          (Variables|Default|SetisLeft true)
          (Variables|Default|SetisDown false)
          (Variables|Default|SetisRight false)
          (Variables|Default|SetisUp false))))
    (else
      (CallFunction|MovetoDirection)
      (goto _label))))

(event EventBeginPlay)

(fn ConstructionScript)