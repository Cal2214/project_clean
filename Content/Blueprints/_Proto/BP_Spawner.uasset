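; BP_Spawner is a prototype actor that spawns BP_Dirt actors at its own transform over time.
; BeginPlay stores the first BP_Dirt found in the level, unused elsewhere here, then spawns one immediately.
; Tick keeps calling RanSpawn, whose latent Delay ignores calls while pending, creating a repeating random wait of seconds.
; After each wait a coin flip decides whether another spawns, adjusted for collision or skipped if blocked.
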(event Custom|DirtRef
  (bind _outactors (Actor|GetAllActorsOfClass "/Game/Blueprints/_Proto/BP_Dirt.BP_Dirt_C"))
  (Variables|Default|SetBP_Dirt (Utilities|Array|Get(acopy) _outactors)))

(event Custom|InitSpawn
  (Game|SpawnActorfromClass "/Game/Blueprints/_Proto/BP_Dirt.BP_Dirt_C" (Transformation|GetActorTransform self) "AdjustIfPossibleButDontSpawnIfColliding" "MultiplyWithRoot" 0 0))

(event Custom|RanSpawn
  (bind _output_get (Variables|Default|SetDelayTime (Math|Random|RandomFloatinRange 2.0 2e+01)))
  (Utilities|FlowControl|Delay _output_get)
  (if (Math|Random|RandomBool)
    (Game|SpawnActorfromClass "/Game/Blueprints/_Proto/BP_Dirt.BP_Dirt_C" (Transformation|GetActorTransform self) "AdjustIfPossibleButDontSpawnIfColliding" "MultiplyWithRoot" 0 0)))

(event EventBeginPlay
  (CallFunction|DirtRef)
  (CallFunction|InitSpawn))

(event EventTick
  (params (DeltaSeconds :type Float%20%28single-precision%29))
  (CallFunction|RanSpawn))

(fn ConstructionScript)