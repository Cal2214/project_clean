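; Prototype pickup that grants either a speed or a size power-up to players and AI.
; On BeginPlay it randomly picks one type, setting its flag and a cube mesh with a type-specific material.
; On sphere overlap, it passes the flags to a player or AI not at max power-ups, then destroys itself.
; AI collectors are also flagged as holding a power-up and notified.
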(event OnComponentBeginOverlap(Sphere)
  (params (OverlappedComponent :type Primitive%20Component%20Object%20Reference) (OtherActor :type Actor%20Object%20Reference) (OtherComp :type Primitive%20Component%20Object%20Reference) (OtherBodyIndex :type Integer) (bFromSweep :type Boolean) (SweepResult :type Hit%20Result%20Structure%20%28by%20ref%29))
  (Utilities|FlowControl|Sequence
    (:then_0
      (bind _asbp_proto_player (Utilities|Casting|CastToBP_protoPlayer OtherActor))
      (if (not (Variables|/Game/Blueprints/_Proto/BP_protoPlayer.BP_protoPlayer_C|GethasMaxPowerup _asbp_proto_player))
        (Default|GetPowerUp _asbp_proto_player (Variables|Default|GetisSpeed) (Variables|Default|GetisSize))
        (Variables|Default|SetisSpeed false)
        (Variables|Default|SetisSize false)
        (Actor|DestroyActor)))
    (:then_1
      (bind _asbp_proto_ai (Utilities|Casting|CastToBP_protoAI OtherActor))
      (if (not (Variables|/Game/Blueprints/_Proto/BP_protoAI.BP_protoAI_C|GethasMaxPowerUp _asbp_proto_ai))
        (Default|GetPowerup _asbp_proto_ai (Variables|Default|GetisSpeed) (Variables|Default|GetisSize))
        (Variables|/Game/Blueprints/_Proto/BP_protoAI.BP_protoAI_C|SethasPowerUP _asbp_proto_ai true)
        (Default|NotiPowerUp _asbp_proto_ai)
        (Variables|Default|SetisSpeed false)
        (Variables|Default|SetisSize false)
        (Actor|DestroyActor)))))

(event Custom|RanPowerUp
  (switch int (Math|Random|RandomInteger 2)
    (:0
      (CallFunction|SpeedIncrease))
    (:1
      (CallFunction|SizeIncrease))))

(event Custom|SpeedIncrease
  (bind _staticmesh (Variables|Default|GetStaticMesh))
  (Variables|Default|SetisSpeed true)
  (Components|StaticMesh|SetStaticMesh _staticmesh "/Engine/VREditor/BasicMeshes/SM_Cube_01.SM_Cube_01")
  (Rendering|Material|SetMaterial _staticmesh 0 "/AnimationSharing/AnimSharingBlue.AnimSharingBlue"))

(event Custom|SizeIncrease
  (bind _staticmesh (Variables|Default|GetStaticMesh))
  (Variables|Default|SetisSize true)
  (Components|StaticMesh|SetStaticMesh _staticmesh "/Engine/VREditor/BasicMeshes/SM_Cube_01.SM_Cube_01")
  (Rendering|Material|SetMaterial _staticmesh 0 "/DatasmithContent/Materials/AliasReference.AliasReference"))

(event EventBeginPlay
  (CallFunction|RanPowerUp))

(fn ConstructionScript)