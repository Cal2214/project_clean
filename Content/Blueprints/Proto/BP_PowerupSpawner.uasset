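; BP_PowerupSpawner is a prototype spawner actor that repeatedly drops BP_PowerUp actors at random spots around itself.
; Tick drives a looping Delay of random length that calls SpawnPowerUp each time it completes.
; SpawnPowerUp takes X and Y from random reachable navmesh points within a wide radius and keeps the spawner's height, adjusting for collisions but always spawning.
; A separate PowerupRef event caches the first BP_PowerUp found in the level.
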(event Custom|PowerupRef
  (bind _outactors (Actor|GetAllActorsOfClass "/Game/Blueprints/Proto/BP_PowerUp.BP_PowerUp_C"))
  (Variables|Default|SetBPPowerup (Utilities|Array|Get(acopy) _outactors)))

(event Custom|SpawnPowerUp
  (bind _self self)
  (bind _returnvalue (Transformation|GetActorLocation _self))
  (bind _randomlocation (AI|Navigation|GetRandomReachablePointinRadius (Math|Vector|MakeVector (.x _returnvalue) (.y _returnvalue) 2e+03) 7e+03 0 0))
  (Game|SpawnActorfromClass "/Game/Blueprints/Proto/BP_PowerUp.BP_PowerUp_C" (Math|Transform|MakeTransform (Math|Vector|MakeVector (.x _randomlocation) (.y _randomlocation) (.z _returnvalue)) "0, 0, 0" "1.000000,1.000000,1.000000") "AdjustIfPossibleButAlwaysSpawn" "MultiplyWithRoot" 0 0))

(event EventBeginPlay)

(event EventTick
  (params (DeltaSeconds :type Float%20%28single-precision%29))
  (Utilities|FlowControl|Delay (Math|Random|RandomFloatinRange 2.0 3e+01) :!label _label)
  (CallFunction|SpawnPowerUp)
  (goto _label))

(fn ConstructionScript)