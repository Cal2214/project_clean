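; BP_PowerUp is a prototype pickup actor that hands a power-up to BP_protoPlayer on overlap.
; On BeginPlay it rolls a random type from three, but only the speed boost is implemented, which sets IsSpeed and changes the mesh to a blue cube.
; When the player overlaps the sphere, it passes IsSpeed to the player's GetPowerUp, clears the flag and destroys itself.
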(event OnComponentBeginOverlap(Sphere)
  (params (OverlappedComponent :type Primitive%20Component%20Object%20Reference) (OtherActor :type Actor%20Object%20Reference) (OtherComp :type Primitive%20Component%20Object%20Reference) (OtherBodyIndex :type Integer) (bFromSweep :type Boolean) (SweepResult :type Hit%20Result%20Structure%20%28by%20ref%29))
  (bind _asbp_proto_player (Utilities|Casting|CastToBP_protoPlayer OtherActor))
  (Default|GetPowerUp _asbp_proto_player (Variables|Default|GetisSpeed))
  (Variables|Default|SetisSpeed false)
  (Actor|DestroyActor))

(event Custom|RanPowerUp
  (switch int (Math|Random|RandomInteger 3)
    (:0
      (CallFunction|SpeedIncrease))))

(event Custom|SpeedIncrease
  (bind _staticmesh (Variables|Default|GetStaticMesh))
  (Variables|Default|SetisSpeed true)
  (Components|StaticMesh|SetStaticMesh _staticmesh "/Engine/VREditor/BasicMeshes/SM_Cube_01.SM_Cube_01")
  (Rendering|Material|SetMaterial _staticmesh 0 "/AnimationSharing/AnimSharingBlue.AnimSharingBlue"))

(event EventBeginPlay
  (CallFunction|RanPowerUp))

(fn ConstructionScript)